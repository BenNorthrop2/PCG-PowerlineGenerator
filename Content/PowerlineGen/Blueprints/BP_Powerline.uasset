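; Procedural powerline actor that builds poles and hanging cables along a spline in the construction script.
; SpawnPosts adds pole meshes per spline point or through a distance-based mode, then calls SpawnCables.
; SpawnCables links same-named sockets on consecutive poles with cable components, setting length from socket distance and physical properties from CableInfoSettings.
; It also stores and prints an incoming power current value and returns it through GetPowerOutputCurrent.
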(event `self.ReceiveBeginPlay`)

(event `/Game/PowerlineGen/Blueprints/Data/BPI_PowelinePower.GetPowerInputCurrent`
  (params (PowerCurrent :type "Float (double-precision)"))
  (bind _output_get (set `self.PowerCurrrent` PowerCurrent))
  (`KismetSystemLibrary.PrintString` (`KismetStringLibrary.Conv_DoubleToString` _output_get)))

(fn `GetPowerOutputCurrent`
  (returns (PowerOutput :type "Float (double-precision)"))
  (return (`self.PowerCurrrent`)))

(fn `SetCableValues`
  (params (`Cable Info Settings` :type "/Game/PowerlineGen/Blueprints/Data/Structs/F_CableInfo Structure"))
  (bind (_cable_ref _positiononspline _cablesocketname _cablelength _cableiterrations _cablestiffness _cablewidth _cableendpoint) (break `/Game/PowerlineGen/Blueprints/Data/Structs/F_CableInfo` `Cable Info Settings`))
  (set `CableComponent.EndLocation` _cableendpoint _cable_ref)
  (set `CableComponent.CableLength` _cablelength _cable_ref)
  (set `CableComponent.SolverIterations` _cableiterrations _cable_ref)
  (set `CableComponent.bEnableStiffness` _cablestiffness _cable_ref)
  (set `CableComponent.CableWidth` _cablewidth _cable_ref))

(fn `SpawnCables`
  (bind _returnvalue (`KismetMathLibrary.InverseTransformLocation` (`self.GetTransform`) (`SceneComponent.GetSocketLocation` (`self.CurrentPoleMesh`) (`self.Current Socket Name`))))
  (bind _output (`|GetArrayItem` (`self.Powerline Poles Array`) (+ (`self.CurrentIndex`) 1)))
  (bind _returnvalue_2 (`KismetMathLibrary.InverseTransformLocation` (`self.GetTransform`) (`SceneComponent.GetSocketLocation` _output (`self.Current Socket Name`))))
  (`KismetArrayLibrary.Array_Clear` (`self.Cable Info Refs`))
  (for (_array_element _array_index) (`self.Powerline Poles Array`)
    (set `self.CurrentPoleMesh` _array_element)
    (set `self.CurrentIndex` _array_index)
    (for _array_element_2 (`SceneComponent.GetAllSocketNames` (`self.CurrentPoleMesh`))
      (set `self.Current Socket Name` _array_element_2)
      (`/Engine/EditorBlueprintResources/StandardMacros.IsValid` _output
        (:`Is Valid`
          (bind _returnvalue_3 (`AddComponent|NODE_AddCableComponent-0` :`RelativeTransform` (`KismetMathLibrary.Conv_VectorToTransform` _returnvalue)))
          (bind _output_get (set `self.CurrentCableRef` _returnvalue_3))
          (`PrimitiveComponent.SetCastShadow` _output_get false)
          (for _array_element_3 (`self.Cable Info Settings`)
            (bind ((`CableSocketName_8_DB8457AD40743BAF03483A9B79BAA109` _cablesocketname) (`CableIterrations_27_86C34B824B025A0B173827BF70789B67` _cableiterrations) (`CableStiffness_19_371D4CDA41D3196617E5ECB7AA674B63` _cablestiffness) (`CableWidth_23_527E520C4F041A075C6B0585CB078835` _cablewidth)) (break `/Game/PowerlineGen/Blueprints/Data/Structs/F_CableInfo` _array_element_3))
            (if (not (== (`self.Current Socket Name`) _cablesocketname))
              (bind _f_cableinfo (make `/Game/PowerlineGen/Blueprints/Data/Structs/F_CableInfo` (`self.CurrentCableRef`) (`self.CurrentIndex`) (`self.Current Socket Name`) (`KismetMathLibrary.VSize` (- _returnvalue _returnvalue_2)) _cableiterrations _cablestiffness _cablewidth _returnvalue_2))
              (`KismetArrayLibrary.Array_Add` (`self.Cable Info Refs`) _f_cableinfo)
              (`self.SetCableValues` _f_cableinfo))))))))

(fn `SpawnPosts`
  (bind _post_spawn_count (`self.Post Spawn Count`))
  (bind _currentindex (`self.CurrentIndex`))
  (bind _spline (`self.Spline`))
  (bind _spline_2 (`self.Spline`))
  (`KismetArrayLibrary.Array_Clear` (`self.Powerline Poles Array`))
  (for _index (range (+ (`SplineComponent.GetNumberOfSplinePoints` (`self.Spline`)) 1))
    (set `self.CurrentIndex` _index)
    (switch `/Game/PowerlineGen/Blueprints/Data/Structs/E_PostSpawnMethod` (`self.Post Spawn Method`)
      (:`NewEnumerator0`
        (if (> _post_spawn_count 1)
          (for _ (range (+ _post_spawn_count 1))
            (bind _returnvalue (`AddComponent|NODE_AddStaticMeshComponent-1` :`RelativeTransform` (`KismetMathLibrary.MakeTransform` (`SplineComponent.GetDirectionAtDistanceAlongSpline` _spline_2 (/ (`SplineComponent.GetSplineLength` _spline_2) (`self.Posts Spawn Distance`)) "Local"))))
            (`StaticMeshComponent.SetStaticMesh` _returnvalue (`self.PowerlineMesh`))
            (`KismetArrayLibrary.Array_Add` (`self.Powerline Poles Array`) _returnvalue))))
      (:`NewEnumerator1`
        ;[0.2354 0.8387 1 0.5] Spawn Posts On Points
        (bind _returnvalue_2 (`AddComponent|NODE_AddStaticMeshComponent-0` :`RelativeTransform` (`KismetMathLibrary.MakeTransform` (`SplineComponent.GetLocationAtSplinePoint` _spline _currentindex "Local") (`SplineComponent.GetRotationAtSplinePoint` _spline _currentindex "Local"))))
        (`StaticMeshComponent.SetStaticMesh` _returnvalue_2 (`self.PowerlineMesh`))
        (`KismetArrayLibrary.Array_Add` (`self.Powerline Poles Array`) _returnvalue_2))))
  (`self.SpawnCables`))

(fn `UserConstructionScript`
  (`self.SpawnPosts`))