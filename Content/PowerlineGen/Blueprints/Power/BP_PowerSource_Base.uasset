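; Base power actor that switches its light on or off according to the power output of nearby powerlines.
; BeginPlay creates a dynamic light material and starts a looping timer for polling.
; SearchForPowerline sphere-traces at a fixed height above the actor's XY position, with debug drawing, and queries hits implementing BPI_PowelinePower.
; Each reading sets light intensity and colour, so the last matching hit wins.
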(event `self.ReceiveBeginPlay`
  (bind _returnvalue (`PrimitiveComponent.CreateDynamicMaterialInstance` (`self.Light`) 0 "/Game/PowerlineGen/Assets/PowerSource/MI_Light.MI_Light" "None"))
  (set `self.LightMaterialRef` _returnvalue)
  (`KismetSystemLibrary.K2_SetTimerDelegate` (`|CreateDelegate` :!event `SearchForPowerline`) 0.5 true))

(event `SearchForPowerline`
  (bind _lightmaterialref (`self.LightMaterialRef`))
  (bind _lightmaterialref_2 (`self.LightMaterialRef`))
  (bind _returnvalue (`KismetMathLibrary.MakeVector` (.x (`self.K2_GetActorLocation`)) (.y (`self.K2_GetActorLocation`)) 600.0))
  (bind _outhits (`KismetSystemLibrary.SphereTraceMulti` :`Start` _returnvalue :`End` _returnvalue :`Radius` 1500.0 :`TraceChannel` "TraceTypeQuery1" :`DrawDebugType` "ForDuration"))
  (for _array_element _outhits
    (bind (_bblockinghit _binitialoverlap _time _distance _location _impactpoint _normal _impactnormal _physmat _hitactor) (`GameplayStatics.BreakHitResult` _array_element))
    (if (`KismetSystemLibrary.DoesImplementInterface` _hitactor "/Game/PowerlineGen/Blueprints/Data/BPI_PowelinePower.BPI_PowelinePower_C")
      (bind _poweroutput (message `/Game/PowerlineGen/Blueprints/Data/BPI_PowelinePower.GetPowerOutputCurrent` _hitactor))
      (if (<= _poweroutput 0.0)
        (`KismetSystemLibrary.PrintString` "Off")
        (`MaterialInstanceDynamic.SetScalarParameterValue` _lightmaterialref_2 "Light_Intensity" 0.0)
        (`MaterialInstanceDynamic.SetVectorParameterValue` _lightmaterialref_2 "Light_Colour" (struct :`A` 1.0))
        (else
          (`KismetSystemLibrary.PrintString` "On")
          (`MaterialInstanceDynamic.SetScalarParameterValue` _lightmaterialref "Light_Intensity" 5.0)
          (`MaterialInstanceDynamic.SetVectorParameterValue` _lightmaterialref "Light_Colour" (struct :`R` 1.0 :`G` 1.0 :`B` 1.0 :`A` 1.0)))))))

(fn `UserConstructionScript`)